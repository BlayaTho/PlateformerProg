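; Grind rail actor that builds spline meshes along its spline in the construction script and runs the player's rail grind.
; DetectPlayerLocation starts grinding at the spline key closest to the player.
; Tick advances that key and, while grinding, sets actor transform just above it and disables player capsule collision.
; Jumped or a hard-coded end key calls JumpOffGrind, restoring collision after a short delay.
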(event `self.ReceiveBeginPlay`
  (bind _asbp_player_base (cast `/Game/Blueprints/BP_PlayerBase` (`GameplayStatics.GetPlayerCharacter` 0)))
  (set `self.As BP Player Base_0` _asbp_player_base))

(event `Jumped`
  (set `self.useGrind` false :!label _label)
  (`/Game/Blueprints/BP_PlayerBase.JumpOffGrind` (`self.As BP Player Base_0`))
  (`KismetSystemLibrary.Delay` 0.2)
  (`PrimitiveComponent.SetCollisionEnabled` (`Character.CapsuleComponent` (`self.As BP Player Base_0`)) "QueryAndPhysics"))

(event `self.ReceiveTick`
  (params (DeltaSeconds :type "Float (single-precision)"))
  (bind _as_bp_player_base_0 (`self.As BP Player Base_0`))
  (bind _spline (`self.Spline`))
  (set `self.KeyPoint` (`KismetMathLibrary.FClamp` (+ (`self.KeyPoint`) (* (`GameplayStatics.GetWorldDeltaSeconds`) 1.0)) 0.0 (`KismetMathLibrary.Conv_IntToDouble` (- (`SplineComponent.GetNumberOfSplinePoints` _spline) 1))))
  (if (`self.useGrind`)
    (set `CharacterMovementComponent.MaxWalkSpeed` 1500.0 (`Character.CharacterMovement` (`self.As BP Player Base_0`)))
    (`self.K2_SetActorLocationAndRotation` (`KismetMathLibrary.MakeVector` (.x (`SplineComponent.GetLocationAtSplineInputKey` _spline (`self.KeyPoint`) "World")) (.y (`SplineComponent.GetLocationAtSplineInputKey` _spline (`self.KeyPoint`) "World")) (+ (.z (`SplineComponent.GetLocationAtSplineInputKey` _spline (`self.KeyPoint`) "World")) 180.0)) (`SplineComponent.GetRotationAtSplineInputKey` (`self.Spline`) (`self.KeyPoint`) "World"))
    (`PrimitiveComponent.SetCollisionEnabled` (`Character.CapsuleComponent` (`self.As BP Player Base_0`)) "NoCollision")
    (set `/Game/Blueprints/BP_PlayerBase.InGrind` false _as_bp_player_base_0)
    (set `/Game/Blueprints/BP_PlayerBase.JumpCount` 0 _as_bp_player_base_0)
    (if (== (`self.KeyPoint`) 5.0)
      (goto _label))))

(event `DetectPlayerLocation`
  (set `self.KeyPoint` (`SplineComponent.FindInputKeyClosestToWorldLocation` (`self.Spline`) (`SceneComponent.K2_GetComponentLocation` (`Character.Mesh` (`GameplayStatics.GetPlayerCharacter` 0)))))
  (set `self.useGrind` true))

(fn `UserConstructionScript`
  (bind _spline (`self.Spline`))
  (for _index (range (+ (- (`SplineComponent.GetNumberOfSplinePoints` (`self.Spline`)) 2) 1))
    (bind _returnvalue (`AddComponent|NODE_AddSplineMeshComponent-0`))
    (bind (_location _tangent) (`SplineComponent.GetLocationAndTangentAtSplinePoint` _spline _index "Local"))
    (bind (_location_2 _tangent_2) (`SplineComponent.GetLocationAndTangentAtSplinePoint` _spline (+ _index 1) "Local"))
    (`SplineMeshComponent.SetStartAndEnd` _returnvalue _location _tangent _location_2 _tangent_2 true)
    (`SceneComponent.K2_AttachToComponent` _returnvalue (`self.Scene`) "None" "KeepRelative" "KeepRelative" "KeepRelative" true)))