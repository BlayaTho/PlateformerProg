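; BP_cible is a target actor (French "cible") that can appear as either a mannequin or a cube.
; The construction script uses the Mannequin flag to show the skeletal mesh or the cube and hide the other.
; A custom event, NewFunction, serves as the hit response: it prints "HIT" and destroys the actor.
; No caller of that event appears in this Blueprint, and BeginPlay does nothing.
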(event `self.ReceiveBeginPlay`)

(event `/Game/Blueprints/NewInterface.NewFunction`
  (`KismetSystemLibrary.PrintString` "HIT")
  (`self.K2_DestroyActor`))

(fn `UserConstructionScript`
  (if (`self.Mannequin?`)
    (`SceneComponent.SetVisibility` (`self.SkeletalMesh`) true false)
    (`SceneComponent.SetVisibility` (`self.Cube`) false false)
    (else
      (`SceneComponent.SetVisibility` (`self.Cube`) true false)
      (`SceneComponent.SetVisibility` (`self.SkeletalMesh`) false false))))