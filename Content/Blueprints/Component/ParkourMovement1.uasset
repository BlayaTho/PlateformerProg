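; Parkour movement component that gives an owning Character wall running, wall jumping and camera tilt.
; After Initialize, a looping timer line-traces to either side; while falling beside a valid wall, launches hold and drive the character along it as gravity eases toward a wall-run value.
; Jump events launch off the wall normal, with timed suppression of new runs after a run ends.
; Tick rolls the control rotation according to wall side.
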(event `WallRunSuppression`
  (`KismetSystemLibrary.K2_ClearTimer` null "ResetWallRunSuppression")
  (set `self.WallRunSuppresed?` false))

(event `LandEvent`
  (`self.WallRunEnd` 0.0)
  (set `self.WallRunSuppresed?` false))

(event `WallRunUpdateEvent`
  (if (not (`self.WallRunSuppresed?`))
    (`self.WallRunUpdate`)))

(event `JumpEvent`
  (`self.WallRunJump`))

(event `Initialize`
  (params (Character :type "Character Object Reference"))
  (bind _output_get (set `self.Character` Character))
  (bind _output_get_2 (set `self.Character Movement` (`Character.CharacterMovement` _output_get)))
  (set `self.DefaultGravity` (`CharacterMovementComponent.GravityScale` _output_get_2))
  (`KismetSystemLibrary.K2_SetTimerDelegate` (delegate `WallRunUpdateEvent`) 0.02 true))

(event `self.ReceiveTick`
  (params (DeltaSeconds :type "Float (single-precision)"))
  (`self.CameraTick`))

(fn `CameraTick`
  (if (`self.WallRunning_L`)
    (`self.CameraTilt` 15.0)
    (elif (`self.WallRunning_R`)
      (`self.CameraTilt` -15.0)
      (else
        (`self.CameraTilt` 0.0)))))

(fn `CameraTilt`
  (params (`Target X (Roll)` :type "Float (double-precision)"))
  (bind _returnvalue (`Controller.GetControlRotation` (`Pawn.GetController` (`self.Character`))))
  (`Controller.SetControlRotation` (`Pawn.GetController` (`self.Character`)) (`KismetMathLibrary.RInterpTo` _returnvalue (`KismetMathLibrary.MakeRotator` `Target X (Roll)` (.pitch _returnvalue) (.yaw _returnvalue)) (`GameplayStatics.GetWorldDeltaSeconds`) 10.0)))

(fn `SupressWallRun`
  (params (delay :type "Float (double-precision)"))
  (set `self.WallRunSuppresed?` true)
  (`KismetSystemLibrary.K2_SetTimer` null "ResetWallRunSuppression" delay))

(fn `WallRunEnd`
  (params (resetTime :type "Float (double-precision)"))
  (if (`self.WallRunning`)
    (set `self.WallRunning` false)
    (set `self.WallRunning_R` false)
    (set `self.WallRunning_L` false)
    (set `CharacterMovementComponent.GravityScale` (`self.DefaultGravity`) (`self.Character Movement`))
    (`self.SupressWallRun` resetTime)))

(fn `WallRunJump`
  (bind (_wallrunnormal_x _wallrunnormal_y) (`KismetMathLibrary.BreakVector` (`self.WallRunNormal`)))
  (bind _wallrunjumpoffforce (`self.WallRunJumpOffForce`))
  (if (`self.WallRunning`)
    (`self.WallRunEnd` 0.35)
    (`Character.LaunchCharacter` (`self.Character`) (`KismetMathLibrary.MakeVector` (* _wallrunjumpoffforce _wallrunnormal_x) (* _wallrunjumpoffforce _wallrunnormal_y) (`self.WallRunJumpHeight`)) false true)))

(fn `WallRunMovement`
  (params (Start :type "Vector Structure") (End :type "Vector Structure") (WallRunDirection :type "Float (double-precision)"))
  (returns (OnWall :type Boolean))
  (bind _character (`self.Character`))
  (bind _outhit (`KismetSystemLibrary.LineTraceSingle` :`Start` Start :`End` End :`TraceChannel` "TraceTypeQuery1" :`DrawDebugType` "ForDuration"))
  (if (`GameplayStatics.BreakHitResult` _outhit)
    (bind (_returnvalue _outvec) (`self.ValidWallRunvector` (`.ImpactNormal` (`GameplayStatics.BreakHitResult` _outhit))))
    (if (and (`NavMovementComponent.IsFalling` (`self.Character Movement`)) _returnvalue)
      (set `self.WallRunNormal` _outvec)
      (`Character.LaunchCharacter` _character (`self.PlayerToWallVector`) false false) ; Stick character to wall
      (`Character.LaunchCharacter` _character (* (`KismetMathLibrary.Cross_VectorVector` (`self.WallRunNormal`) (0.0 0.0 1.0)) (* (`self.WallRunSpeed`) (`local.WallRunDirection`))) true (not (`self.WallRunGravity`))) ; Move forward
      (return true)
      (else
        (return false)))
    (else
      (return false))))

(fn `WallRunUpdate`
  (bind _onwall (`self.WallRunMovement` (`Actor.K2_GetActorLocation` (`self.Character`)) (`self.WallRunEndVectors`) -1.0)) ; right
  (if _onwall
    (set `self.WallRunning` true)
    (set `self.WallRunning_R` true)
    (set `self.WallRunning_L` false)
    (set `CharacterMovementComponent.GravityScale` (`KismetMathLibrary.FInterpTo` (`CharacterMovementComponent.GravityScale` (`self.Character Movement`)) (`self.WallRunTargetGravity`) (`GameplayStatics.GetWorldDeltaSeconds`) 10.0) (`self.Character Movement`) :!label _label)
    (elif (`self.WallRunning_R`)
      (`self.WallRunEnd` 1.0)
      (else
        (bind _onwall_2 (`self.WallRunMovement` (`Actor.K2_GetActorLocation` (`self.Character`)) (`.Left` (`self.WallRunEndVectors`)) 1.0)) ; Left
        (if _onwall_2
          (set `self.WallRunning` true)
          (set `self.WallRunning_R` false)
          (set `self.WallRunning_L` true)
          (goto _label)
          (else
            (`self.WallRunEnd` 1.0)))))))