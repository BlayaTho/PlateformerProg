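; Sword-wielding enemy target that kills the player on sword contact and dies when shot or bounced on.
; Overlap triggers start a looping timer that smoothly yaws it toward the player, and a self-repeating attack montage with a delay while in range.
; The bounce trigger calls the player's Bouncing, while HitboxIA destroys whatever overlaps it.
; Death stops the facing timer, disables collisions, flags Dead and activates sparks, leaving the actor in place.
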(event `self.ReceiveBeginPlay`
  ;[1 1 1] BeginPlay
  (bind _asbp_player_base (cast `/Game/Project_P/Blueprints/BP_PlayerBase` (`GameplayStatics.GetPlayerCharacter` 0)))
  (set `self.As BP Player Base` _asbp_player_base))

(event `self.TriggerCanRotate.OnComponentBeginOverlap`
  (params (OverlappedComponent :type "PrimitiveComponent Object Reference") (OtherActor :type "Actor Object Reference") (OtherComp :type "PrimitiveComponent Object Reference") (OtherBodyIndex :type Integer) (bFromSweep :type Boolean) (SweepResult :type "HitResult Structure (by ref)"))
  ;[0.1146 0.1146 0.1146] Rotation du personnage pour qu'il soit toujours face au player
  (cast `/Game/Project_P/Blueprints/BP_PlayerBase` OtherActor)
  (bind _returnvalue (`KismetSystemLibrary.K2_SetTimerDelegate` (delegate `FacePlayer`) 0.01 true))
  (set `self.TickFacePlayer` _returnvalue))

(event `self.TriggerCanRotate.OnComponentEndOverlap`
  (params (OverlappedComponent :type "PrimitiveComponent Object Reference") (OtherActor :type "Actor Object Reference") (OtherComp :type "PrimitiveComponent Object Reference") (OtherBodyIndex :type Integer))
  ;[0.1146 0.1146 0.1146] Rotation du personnage pour qu'il soit toujours face au player
  (`KismetSystemLibrary.K2_ClearAndInvalidateTimerHandle` (`self.TickFacePlayer`)))

(event `FacePlayer`
  (bind (_returnvalue_roll _returnvalue_pitch _returnvalue_yaw) (`KismetMathLibrary.BreakRotator` (`KismetMathLibrary.RInterpTo` (`self.K2_GetActorRotation`) (`KismetMathLibrary.FindLookAtRotation` (`self.K2_GetActorLocation`) (`self.K2_GetActorLocation` (`self.As BP Player Base`))) (`GameplayStatics.GetWorldDeltaSeconds`) 10.0)))
  ;[0.1146 0.1146 0.1146] Rotation du personnage pour qu'il soit toujours face au player
  (`self.K2_SetActorRotation` (`KismetMathLibrary.MakeRotator` 0.0 0.0 _returnvalue_yaw)))

(event `AttackLoop`
  ;[0.04688 0.04688 0.04688] Detection si le joueur est dans la zone d'attaque et loop si il reste dedans
  (`|PlayMontage` (`self.SkeletalMesh`) "/Game/Project_P/Animation/Mon_Attack_01_Sword.Mon_Attack_01_Sword"
    (:`OnCompleted`
      (`KismetSystemLibrary.RetriggerableDelay` 1.0)
      (if (`self.CanAttack?`)
        (`self.AttackLoop`)))))

(event `self.TriggerCanAttack.OnComponentBeginOverlap`
  (params (OverlappedComponent :type "PrimitiveComponent Object Reference") (OtherActor :type "Actor Object Reference") (OtherComp :type "PrimitiveComponent Object Reference") (OtherBodyIndex :type Integer) (bFromSweep :type Boolean) (SweepResult :type "HitResult Structure (by ref)"))
  ;[0.04688 0.04688 0.04688] Detection si le joueur est dans la zone d'attaque et loop si il reste dedans
  (cast `/Game/Project_P/Blueprints/BP_PlayerBase` OtherActor)
  (set `self.CanAttack?` true)
  (`self.AttackLoop`))

(event `self.TriggerCanAttack.OnComponentEndOverlap`
  (params (OverlappedComponent :type "PrimitiveComponent Object Reference") (OtherActor :type "Actor Object Reference") (OtherComp :type "PrimitiveComponent Object Reference") (OtherBodyIndex :type Integer))
  ;[0.04688 0.04688 0.04688] Detection si le joueur est dans la zone d'attaque et loop si il reste dedans
  (set `self.CanAttack?` false))

(event `/Game/Project_P/Blueprints/Interface/BPI_shoot.ShootSomething`
  ;[0.1719 0.1719 0.1719] Mort de l'IA par le rebond ou la detection du tir
  (`self.Death` :!label _label))

(event `self.Trigger_Bounce.OnComponentBeginOverlap`
  (params (OverlappedComponent :type "PrimitiveComponent Object Reference") (OtherActor :type "Actor Object Reference") (OtherComp :type "PrimitiveComponent Object Reference") (OtherBodyIndex :type Integer) (bFromSweep :type Boolean) (SweepResult :type "HitResult Structure (by ref)"))
  ;[0.1719 0.1719 0.1719] Mort de l'IA par le rebond ou la detection du tir
  (bind _asbp_player_base (cast `/Game/Project_P/Blueprints/BP_PlayerBase` OtherActor))
  (`/Game/Project_P/Blueprints/BP_PlayerBase.Bouncing` _asbp_player_base)
  (goto _label))

(event `self.HitboxIA.OnComponentBeginOverlap`
  (params (OverlappedComponent :type "PrimitiveComponent Object Reference") (OtherActor :type "Actor Object Reference") (OtherComp :type "PrimitiveComponent Object Reference") (OtherBodyIndex :type Integer) (bFromSweep :type Boolean) (SweepResult :type "HitResult Structure (by ref)"))
  ;[0.1719 0.1719 0.1719] Mort de l'IA par le rebond ou la detection du tir
  (`self.K2_DestroyActor` OtherActor))

(event `self.Trigger_Sword.OnComponentBeginOverlap`
  (params (OverlappedComponent :type "PrimitiveComponent Object Reference") (OtherActor :type "Actor Object Reference") (OtherComp :type "PrimitiveComponent Object Reference") (OtherBodyIndex :type Integer) (bFromSweep :type Boolean) (SweepResult :type "HitResult Structure (by ref)"))
  ;[0.1719 0.1719 0.1719] Mort de l'IA par le rebond ou la detection du tir
  ;;[1 1 1] Detection degat sur le joueur avec le trigger sur l'épée
  (bind _asbp_player_base (cast `/Game/Project_P/Blueprints/BP_PlayerBase` OtherActor))
  (`self.K2_DestroyActor` _asbp_player_base))

(event `Death`
  ;[0.1354 0.1354 0.1354] Event Death
  (`KismetSystemLibrary.K2_ClearAndInvalidateTimerHandle` (`self.TickFacePlayer`))
  (`PrimitiveComponent.SetCollisionEnabled` (`self.TriggerAssistVisee`) "NoCollision")
  (`PrimitiveComponent.SetCollisionEnabled` (`self.TriggerCanRotate`) "NoCollision")
  (`PrimitiveComponent.SetCollisionEnabled` (`self.Sword`) "NoCollision")
  (`PrimitiveComponent.SetCollisionEnabled` (`self.SkeletalMesh`) "NoCollision")
  (`PrimitiveComponent.SetCollisionEnabled` (`self.TriggerCanAttack`) "NoCollision")
  (`PrimitiveComponent.SetCollisionEnabled` (`self.HitboxIA`) "NoCollision")
  (`PrimitiveComponent.SetCollisionEnabled` (`self.Trigger_Sword`) "NoCollision")
  (`PrimitiveComponent.SetCollisionEnabled` (`self.Trigger_Bounce`) "NoCollision")
  (set `self.Dead` true)
  (`ActorComponent.Activate` (`self.PS_FX_Sparks`) false))

(fn `UserConstructionScript`)