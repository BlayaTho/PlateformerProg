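; BP_WallRun is a static mesh wall piece, named for wall running, with selectable orange, gray and black looks.
; The construction script checks the three color booleans in that order, clears the other two and applies the matching material and greeble cube mesh.
; Gray and black share a material but differ in mesh, while orange and gray share a mesh.
; It has no runtime logic.
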(fn `UserConstructionScript`
  (bind _staticmeshcomponent0 (`self.StaticMeshComponent0`))
  (bind _staticmeshcomponent0_2 (`self.StaticMeshComponent0`))
  (`|ExecutionSequence`
    (:`then_0`
      (if (`self.isOrange?`)
        (set `self.isGray?` false)
        (set `self.isBlack?` false)
        (`PrimitiveComponent.SetMaterial` _staticmeshcomponent0 0 "/Game/PolygonScifi/Materials/M_PolygonScifi_01_A1.M_PolygonScifi_01_A1")
        (`StaticMeshComponent.SetStaticMesh` _staticmeshcomponent0_2 "/Game/PolygonScifi/Meshes/Environments/SM_Env_Greeble_Cube_01.SM_Env_Greeble_Cube_01")))
    (:`then_1`
      (if (`self.isGray?`)
        (set `self.isOrange?` false)
        (set `self.isBlack?` false)
        (`PrimitiveComponent.SetMaterial` _staticmeshcomponent0 0 "/Game/PolygonScifi/Materials/M_PolygonScifi_01_A.M_PolygonScifi_01_A")
        (`StaticMeshComponent.SetStaticMesh` _staticmeshcomponent0_2 "/Game/PolygonScifi/Meshes/Environments/SM_Env_Greeble_Cube_01.SM_Env_Greeble_Cube_01")))
    (:`then_2`
      (if (`self.isBlack?`)
        (set `self.isGray?` false)
        (set `self.isOrange?` false)
        (`PrimitiveComponent.SetMaterial` _staticmeshcomponent0 0 "/Game/PolygonScifi/Materials/M_PolygonScifi_01_A.M_PolygonScifi_01_A")
        (`StaticMeshComponent.SetStaticMesh` _staticmeshcomponent0_2 "/Game/PolygonScifi/Meshes/Environments/SM_Env_Greeble_Cube_02.SM_Env_Greeble_Cube_02")))))