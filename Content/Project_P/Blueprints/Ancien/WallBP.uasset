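; WallBP is a wall actor with a selectable prototyping look, configured entirely in its Construction Script.
; It applies the CastShadow setting to the static mesh, then checks five style booleans to set material slot 0 to a grid or solid material.
; Each matching branch clears the other flags, so the first enabled one in sequence order wins.
; The event graph has no active logic.
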(fn `UserConstructionScript`
  (bind _staticmeshcomponent0 (`self.StaticMeshComponent0`))
  (`PrimitiveComponent.SetCastShadow` (`self.StaticMeshComponent0`) (`self.CastShadow?`))
  (`|ExecutionSequence`
    (:`then_0`
      (if (`self.TopDark?`)
        (`PrimitiveComponent.SetMaterial` _staticmeshcomponent0 0 "/Game/LevelPrototyping/Materials/MI_PrototypeGrid_TopDark.MI_PrototypeGrid_TopDark")
        (set `self.TopDark?` true)
        (set `self.GrayGrid?` false)
        (set `self.SolidBlue?` false)
        (set `self.SolidGray?` false)
        (set `self.GreenGrid?` false)))
    (:`then_1`
      (if (`self.GrayGrid?`)
        (`PrimitiveComponent.SetMaterial` _staticmeshcomponent0 0 "/Game/LevelPrototyping/Materials/M_PrototypeGrid.M_PrototypeGrid")
        (set `self.TopDark?` false)
        (set `self.GrayGrid?` true)
        (set `self.SolidBlue?` false)
        (set `self.SolidGray?` false)
        (set `self.GreenGrid?` false)))
    (:`then_2`
      (if (`self.SolidBlue?`)
        (`PrimitiveComponent.SetMaterial` _staticmeshcomponent0 0 "/Game/LevelPrototyping/Materials/MI_Solid_Blue.MI_Solid_Blue")
        (set `self.TopDark?` false)
        (set `self.GrayGrid?` false)
        (set `self.SolidBlue?` true)
        (set `self.SolidGray?` false)
        (set `self.GreenGrid?` false)))
    (:`then_3`
      (if (`self.SolidGray?`)
        (`PrimitiveComponent.SetMaterial` _staticmeshcomponent0 0 "/Game/LevelPrototyping/Materials/M_Solid.M_Solid")
        (set `self.TopDark?` false)
        (set `self.GrayGrid?` false)
        (set `self.SolidBlue?` false)
        (set `self.SolidGray?` true)
        (set `self.GreenGrid?` false)))
    (:`then_4`
      (if (`self.GreenGrid?`)
        (`PrimitiveComponent.SetMaterial` _staticmeshcomponent0 0 "/Game/LevelPrototyping/Materials/MI_PrototypeGrid_Green.MI_PrototypeGrid_Green")
        (set `self.TopDark?` false)
        (set `self.GrayGrid?` false)
        (set `self.SolidBlue?` false)
        (set `self.SolidGray?` false)
        (set `self.GreenGrid?` true)))))