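; BP_Cube is a test moving cube that travels along the first BP_SplinePath spline and carries the player.
; On BeginPlay, a timeline scaled by TimeToCompleteS drives the cube's location and rotation by distance along the spline.
; An overlapping BP_PlayerBase is teleported to the Scene component, then receives the cube's velocity every Tick.
; Leaving the box stops this and clamps the player's X and Y velocity.
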(event `self.ReceiveBeginPlay`
  (bind _returnvalue (`GameplayStatics.GetActorOfClass` "/Game/Project_P/Blueprints/Ancien/testSpline/BP_SplinePath.BP_SplinePath_C"))
  (set `self.SplineRef` _returnvalue)
  (`self.Move Object`))

(event `Move Object`
  (bind _spline (`/Game/Project_P/Blueprints/Ancien/testSpline/BP_SplinePath.Spline` (`self.SplineRef`)))
  (`TimelineComponent.SetPlayRate` (`self.MoveObjectT`) (/ 1.0 (`self.TimeToComplete (s)`)))
  (bind (_direction _movetrack) (`Timeline|MoveObjectT`)
    (:`Update`
      (bind _returnvalue (`KismetMathLibrary.Lerp` 0.0 (`SplineComponent.GetSplineLength` (`/Game/Project_P/Blueprints/Ancien/testSpline/BP_SplinePath.Spline` (`self.SplineRef`))) _movetrack))
      (`self.K2_SetActorTransform` (`KismetMathLibrary.MakeTransform` (`SplineComponent.GetLocationAtDistanceAlongSpline` _spline _returnvalue "World") (`SplineComponent.GetRotationAtDistanceAlongSpline` _spline _returnvalue "Local"))))))

(event `self.ReceiveTick`
  (params (DeltaSeconds :type "Float (single-precision)"))
  (if (`self.Velocited`)
    (set `MovementComponent.Velocity` (`self.GetVelocity`) (`Character.CharacterMovement` (`self.As BP Player Base`)))))

(event `self.Box.OnComponentBeginOverlap`
  (params (OverlappedComponent :type "PrimitiveComponent Object Reference") (OtherActor :type "Actor Object Reference") (OtherComp :type "PrimitiveComponent Object Reference") (OtherBodyIndex :type Integer) (bFromSweep :type Boolean) (SweepResult :type "HitResult Structure (by ref)"))
  (bind _asbp_player_base (cast `/Game/Project_P/Blueprints/BP_PlayerBase` OtherActor))
  (bind _output_get (set `self.As BP Player Base` _asbp_player_base))
  (`self.K2_SetActorLocation` _output_get (`SceneComponent.K2_GetComponentLocation` (`self.Scene`)) false false)
  (set `self.Velocited` true))

(event `self.Box.OnComponentEndOverlap`
  (params (OverlappedComponent :type "PrimitiveComponent Object Reference") (OtherActor :type "Actor Object Reference") (OtherComp :type "PrimitiveComponent Object Reference") (OtherBodyIndex :type Integer))
  (bind _asbp_player_base (cast `/Game/Project_P/Blueprints/BP_PlayerBase` OtherActor))
  (bind _charactermovement (`Character.CharacterMovement` _asbp_player_base))
  (bind (_velocity_x _velocity_y _velocity_z) (`KismetMathLibrary.BreakVector` (`MovementComponent.Velocity` _charactermovement)))
  (set `MovementComponent.Velocity` (`KismetMathLibrary.MakeVector` (`KismetMathLibrary.FClamp` _velocity_x -600.0 600.0) (`KismetMathLibrary.FClamp` _velocity_y -600.0 600.0) _velocity_z) _charactermovement)
  (set `self.Velocited` false))

(fn `UserConstructionScript`)