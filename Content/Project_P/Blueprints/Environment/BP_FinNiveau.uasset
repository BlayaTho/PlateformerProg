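; End-of-level trigger actor that stops the level timer and lets the player choose the next map.
; On BeginPlay it adds the W_EndLevel timer widget to the viewport and caches the BP_PlayerBase character.
; Any Box overlap, unfiltered, stops the timer, calls EndUI and moves input from the character to this actor.
; IA_Shoot then opens NextLevelName, while IA_Aim opens LevelName.
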(event `self.ReceiveBeginPlay`
  (bind _returnvalue (`|CreateWidget` "/Game/Project_P/Blueprints/UI/W_EndLevel.W_EndLevel_C"))
  (bind _output_get (set `self.w_timer` _returnvalue))
  (`UserWidget.AddToViewport` _output_get 0)
  (bind _asbp_player_base (cast `/Game/Project_P/Blueprints/Player/BP_PlayerBase` (`GameplayStatics.GetPlayerCharacter` 0)))
  (set `self.As BP Player Base` _asbp_player_base))

(event `self.Box.OnComponentBeginOverlap`
  (params (OverlappedComponent :type "PrimitiveComponent Object Reference") (OtherActor :type "Actor Object Reference") (OtherComp :type "PrimitiveComponent Object Reference") (OtherBodyIndex :type Integer) (bFromSweep :type Boolean) (SweepResult :type "HitResult Structure (by ref)"))
  (bind _returnvalue (`GameplayStatics.GetPlayerController` 0))
  (bind _w_timer (`self.w_timer`))
  (set `/Game/Project_P/Blueprints/UI/W_EndLevel.StopTimer?` true _w_timer)
  (`/Game/Project_P/Blueprints/UI/W_EndLevel.EndUI` _w_timer)
  (`self.DisableInput` (`self.As BP Player Base`) _returnvalue)
  (`self.EnableInput` _returnvalue))

(event `EnhancedInput|/Game/FirstPerson/Input/Actions/IA_Shoot`
  (params (ActionValue :type Boolean) (ElapsedSeconds :type "Float (double-precision)") (TriggeredSeconds :type "Float (double-precision)") (InputAction :type "InputAction Object Reference" :default "/Game/FirstPerson/Input/Actions/IA_Shoot.IA_Shoot"))
  (:`Started`
    (`GameplayStatics.OpenLevel` (`self.NextLevelName`))))

(event `EnhancedInput|/Game/Project_P/Blueprints/Inputs/Actions/IA_Aim`
  (params (ActionValue :type Boolean) (ElapsedSeconds :type "Float (double-precision)") (TriggeredSeconds :type "Float (double-precision)") (InputAction :type "InputAction Object Reference" :default "/Game/Project_P/Blueprints/Inputs/Actions/IA_Aim.IA_Aim"))
  (:`Started`
    (`GameplayStatics.OpenLevel` (`self.Level Name`))))

(fn `UserConstructionScript`)