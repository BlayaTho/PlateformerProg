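; Grind rail actor that carries the player along a spline, with spline meshes built per segment in the construction script.
; DetectPlayerLocation starts the grind at the spline key closest to the player's mesh.
; Tick advances that key by grind speed, snapping the player above the spline with capsule collision off and grind flags set.
; Jumped, or reaching a hardcoded key, ends the grind through JumpOffGrind and restores collision after a short delay.
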(event `self.ReceiveBeginPlay`
  (bind _asbp_player_base (cast `/Game/Project_P/Blueprints/BP_PlayerBase` (`GameplayStatics.GetPlayerCharacter` 0)))
  (set `self.As BP Player Base` _asbp_player_base))

(event `Jumped`
  (bind _as_bp_player_base (`self.As BP Player Base`))
  (set `self.useGrind` false :!label _label)
  (`/Game/Project_P/Blueprints/BP_PlayerBase.JumpOffGrind` _as_bp_player_base)
  (`KismetSystemLibrary.Delay` 0.2)
  (`PrimitiveComponent.SetCollisionEnabled` (`Character.CapsuleComponent` _as_bp_player_base) "QueryAndPhysics"))

(event `self.ReceiveTick`
  (params (DeltaSeconds :type "Float (single-precision)"))
  (bind _as_bp_player_base (`self.As BP Player Base`))
  (bind _as_bp_player_base_2 (`self.As BP Player Base`))
  (bind _spline (`self.Spline`))
  (set `self.KeyPoint` (`KismetMathLibrary.FClamp` (+ (`self.KeyPoint`) (* (`GameplayStatics.GetWorldDeltaSeconds`) (`self.SpeedGrind`))) 0.0 (`KismetMathLibrary.Conv_IntToDouble` (- (`SplineComponent.GetNumberOfSplinePoints` _spline) 1))))
  (if (`self.useGrind`)
    (set `CharacterMovementComponent.MaxWalkSpeed` 1500.0 (`Character.CharacterMovement` _as_bp_player_base_2))
    (`self.K2_SetActorLocationAndRotation` (`self.As BP Player Base`) (`KismetMathLibrary.MakeVector` (.x (`SplineComponent.GetLocationAtSplineInputKey` _spline (`self.KeyPoint`) "World")) (.y (`SplineComponent.GetLocationAtSplineInputKey` _spline (`self.KeyPoint`) "World")) (+ (.z (`SplineComponent.GetLocationAtSplineInputKey` _spline (`self.KeyPoint`) "World")) 180.0)) (`SplineComponent.GetRotationAtSplineInputKey` (`self.Spline`) (`self.KeyPoint`) "World") false false)
    (`PrimitiveComponent.SetCollisionEnabled` (`Character.CapsuleComponent` _as_bp_player_base_2) "NoCollision")
    (set `/Game/Project_P/Blueprints/BP_PlayerBase.InGrind` true _as_bp_player_base)
    (set `/Game/Project_P/Blueprints/BP_PlayerBase.CantmoveGrind` true _as_bp_player_base)
    (set `/Game/Project_P/Blueprints/BP_PlayerBase.JumpCount` 0 _as_bp_player_base)
    (if (== (`self.KeyPoint`) 5.0)
      (goto _label))))

(event `DetectPlayerLocation`
  (set `self.KeyPoint` (`SplineComponent.FindInputKeyClosestToWorldLocation` (`self.Spline`) (`SceneComponent.K2_GetComponentLocation` (`Character.Mesh` (`GameplayStatics.GetPlayerCharacter` 0)))))
  (set `self.useGrind` true))

(fn `UserConstructionScript`
  (bind _spline (`self.Spline`))
  (for _index (range (+ (- (`SplineComponent.GetNumberOfSplinePoints` (`self.Spline`)) 2) 1))
    (bind _returnvalue (`AddComponent|NODE_AddSplineMeshComponent-0`))
    (bind (_location _tangent) (`SplineComponent.GetLocationAndTangentAtSplinePoint` _spline _index "Local"))
    (bind (_location_2 _tangent_2) (`SplineComponent.GetLocationAndTangentAtSplinePoint` _spline (+ _index 1) "Local"))
    (`SplineMeshComponent.SetStartAndEnd` _returnvalue _location _tangent _location_2 _tangent_2 true)
    (`SceneComponent.K2_AttachToComponent` _returnvalue (`self.Scene`) "None" "KeepRelative" "KeepRelative" "KeepRelative" true)))