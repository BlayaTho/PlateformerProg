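; Game mode that handles player death and respawn for BP_PlayerBase.
; On BeginPlay and after each respawn, it binds to the player's OnDestroyed, creates the death widget and adds a new controls widget to the viewport.
; When the player is destroyed, it briefly shows the death widget, spawns a replacement at TransformRespawn, possesses it and calls Respawn to rebind.
; Earlier controls widgets are never removed here.
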(event `Respawn`
  (bind _asbp_player_base (cast `/Game/Project_P/Blueprints/Player/BP_PlayerBase` (`GameplayStatics.GetPlayerCharacter` 0) :!label _label))
  (add `self.OnDestroyed` _asbp_player_base (delegate `OnDestroyed_`))
  (bind _returnvalue (`|CreateWidget` "/Game/Project_P/Blueprints/UI/W_Death.W_Death_C"))
  (set `self.W_Death` _returnvalue)
  (bind _returnvalue_2 (`|CreateWidget` "/Game/Project_P/Blueprints/UI/W_Controls.W_Controls_C"))
  (`UserWidget.AddToViewport` _returnvalue_2 0))

(event `self.ReceiveBeginPlay`
  (goto _label))

(event `OnDestroyed_` :!signature `self.OnDestroyed`
  (params (DestroyedActor :type "Actor Object Reference"))
  (bind _w_death (`self.W_Death`))
  (`UserWidget.AddToViewport` _w_death 0)
  (`KismetSystemLibrary.Delay` 0.8)
  (`Widget.RemoveFromParent` _w_death)
  (bind _returnvalue (`|SpawnActorFromClass` "/Game/Project_P/Blueprints/Player/BP_PlayerBase.BP_PlayerBase_C" (`self.TransformRespawn`) "AdjustIfPossibleButAlwaysSpawn" "MultiplyWithRoot" null null))
  (`Controller.Possess` (`GameplayStatics.GetPlayerController` 0) _returnvalue)
  (`self.Respawn`))

(fn `UserConstructionScript`)